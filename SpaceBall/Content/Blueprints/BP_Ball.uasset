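; BP_Ball is a ball actor that plays impact sounds when its Sphere component hits something.
; On a hit it plays the Audio component if the other actor is the player pawn, otherwise Audio1.
; Neither sound starts while either audio component is still playing, so repeated hits do not overlap or restart them.
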(event OnComponentHit(Sphere)
  (params (HitComponent :type Primitive%20Component%20Object%20Reference) (OtherActor :type Actor%20Object%20Reference) (OtherComp :type Primitive%20Component%20Object%20Reference) (NormalImpulse :type Vector :default "0, 0, 0") (Hit :type Hit%20Result%20Structure%20%28by%20ref%29))
  (if (and (Math|Boolean|NotEqual(Boolean) (Audio|Components|Audio|IsPlaying (Variables|Default|GetAudio1)) true) (Math|Boolean|NotEqual(Boolean) (Audio|Components|Audio|IsPlaying (Variables|Default|GetAudio)) true))
    (if (== OtherActor (Game|Player|GetPlayerPawn 0))
      (Audio|Components|Audio|Play (Variables|Default|GetAudio) 0.0)
      (else
        (Audio|Components|Audio|Play (Variables|Default|GetAudio1) 0.0)))))

(fn ConstructionScript)