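; VR player pawn for SpaceBall that flies by hand-held thrusters, with paddle components and eye-level tracking origin.
; Each trigger axis pushes the pawn opposite its controller's forward vector through FloatingPawnMovement, with higher acceleration when both thrusters are active.
; Press inputs act as left mouse clicks on each hand's widget interaction component.
; BeginPlay calls IgnoreActorWhenMoving on the left paddle only; the right paddle's call is disconnected.
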(event EventBeginPlay
  (Class|HeadMountedDisplayFunctionLibrary|SetTrackingOrigin "Eye")
  (Collision|IgnoreActorwhenMoving (Variables|Default|GetPaddleL) 0 true))

(event Input|ActionEvents|InputActionLeftPress
  (params (Key :type Key%20Structure :default "None"))
  (bind _widgetinteractionl (Variables|Default|GetWidgetInteractionL))
  (:Pressed
    (Class|WidgetInteractionComponent|PressPointerKey _widgetinteractionl "LeftMouseButton"))
  (:Released
    (Class|WidgetInteractionComponent|ReleasePointerKey _widgetinteractionl "LeftMouseButton")))

(event Input|ActionEvents|InputActionRightPress
  (params (Key :type Key%20Structure :default "None"))
  (bind _widgetinteractionr (Variables|Default|GetWidgetInteractionR))
  (:Pressed
    (Class|WidgetInteractionComponent|PressPointerKey _widgetinteractionr "LeftMouseButton"))
  (:Released
    (Class|WidgetInteractionComponent|ReleasePointerKey _widgetinteractionr "LeftMouseButton")))

(event Input|AxisEvents|InputAxisLeftThrust
  (params (AxisValue :type Float%20%28single-precision%29))
  (bind _floatingpawnmovement (Variables|Default|GetFloatingPawnMovement))
  ;[1 1 1] LeftThrust
  (if (> AxisValue 0.5)
    (Variables|Default|SetLeftActive true)
    (if (Variables|Default|GetRightActive)
      (Variables|/Script/Engine.FloatingPawnMovement|SetAcceleration _floatingpawnmovement 5e+01)
      (else
        (Variables|/Script/Engine.FloatingPawnMovement|SetAcceleration _floatingpawnmovement 2e+01)))
    (else
      (Variables|Default|SetLeftActive false)))
  (Pawn|Input|AddMovementInput (* (Math|Vector|GetForwardVector (Variables|Default|GetMotionControllerL)) -1.0) AxisValue false))

(event Input|AxisEvents|InputAxisRightThrust
  (params (AxisValue :type Float%20%28single-precision%29))
  (bind _floatingpawnmovement (Variables|Default|GetFloatingPawnMovement))
  ;[1 1 1] RightThrust
  (if (> AxisValue 0.5)
    (Variables|Default|SetRightActive true)
    (if (Variables|Default|GetLeftActive)
      (Variables|/Script/Engine.FloatingPawnMovement|SetAcceleration _floatingpawnmovement 5e+01)
      (else
        (Variables|/Script/Engine.FloatingPawnMovement|SetAcceleration _floatingpawnmovement 2e+01)))
    (else
      (Variables|Default|SetRightActive false)))
  (Pawn|Input|AddMovementInput (* (Math|Vector|GetForwardVector (Variables|Default|GetMotionControllerR)) -1.0) AxisValue false))

(fn ConstructionScript)